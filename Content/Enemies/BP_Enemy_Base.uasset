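; Base enemy character Blueprint that provides attack, patrol route and movement speed functions.
; Attack plays the attack montage on the mesh and fires OnAttackEnd whether the montage completes or is interrupted.
; GetPatrolRoute exposes the stored route, while SetMovementSpeed maps an Idle, Walk or Run state to the character movement's max walk speed and returns the applied value.
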(event `self.ReceiveBeginPlay`)

(event `Attack`
  (`|PlayMontage` (`self.Mesh`) (`self.AttackMontage`)
    (:`OnCompleted`
      _)
    (:`OnInterrupted`
      _))
  (`self.OnAttackEnd`))

(fn `GetPatrolRoute`
  (returns (PatrolRoute :type "/Game/Enemies/AI/BP_Patrol_Route Object Reference"))
  (return (`self.PatrolRoute`)))

(fn `SetMovementSpeed`
  (params (Speed :type "/Game/Blueprints/Enums/E_MovementSpeed Enum" :default "NewEnumerator0"))
  (returns (SpeedValue :type "Float (double-precision)"))
  (bind _output_get (set `CharacterMovementComponent.MaxWalkSpeed` (select `/Game/Blueprints/Enums/E_MovementSpeed` Speed :`NewEnumerator1` 300.0 :`NewEnumerator2` 700.0) (`self.CharacterMovement`)))
  (return _output_get))

(fn `UserConstructionScript`)