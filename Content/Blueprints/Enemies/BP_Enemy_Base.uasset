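; Base enemy character with health, a melee attack, death handling, a patrol route getter and selectable movement speeds.
; A health component receives damage and drives death and the overhead widget health bar, which turns toward the camera every tick.
; Attack plays a montage and signals when it ends or is interrupted.
; A socket-based sphere trace damages only the player, once per attack, using a list of already-hit actors.
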(event `self.ReceiveBeginPlay`
  ; BeginPlay
  (`|ExecutionSequence`
    (:`then_0`
      (bind _aswb_enemy (cast `/Game/UI/WB_Enemy` (`WidgetComponent.GetWidget` (`self.Widget`))))
      (set `self.HUDWidget` _aswb_enemy))
    (:`then_1`
      (`self.BindUIEvents`))))

(event `Death`
  ; Death Logic
  (`self.PlayAnimMontage` (`self.DeathMontage`))
  (`PrimitiveComponent.SetCollisionEnabled` (`self.CapsuleComponent`) "NoCollision")
  (set `self.HUDWidget` null)
  (`ActorComponent.K2_DestroyComponent` (`self.Widget`)))

(event `/Game/Blueprints/Interfaces/BPI_Damageable.TakeDamage`
  (params (Damage :type "Float (double-precision)") (DamageDealer :type "Actor Object Reference"))
  ; On Damaged
  (bind _bpc_healthcomponent (`self.BPC_HealthComponent`)
    (:`then`
      (`/Game/Blueprints/Components/BPC_HealthComponent.Decrease Health` _bpc_healthcomponent Damage DamageDealer))
    (:`else`)))

(event `/Game/Blueprints/Enemies/AI/BPI_EnemyAI.BasicAttackTrace`
  (bind _returnvalue (`GameplayStatics.GetPlayerCharacter` 0))
  (bind _returnvalue_2 (`SceneComponent.GetSocketLocation` (`self.Mesh`) (`self.AttackPointSocketName`)))
  ; Attack Logic
  ;; Attack Trace
  (bind (_outhit _returnvalue_3) (`KismetSystemLibrary.SphereTraceSingle` :`Start` _returnvalue_2 :`End` (- _returnvalue_2 (* (`self.GetActorForwardVector`) 15.0)) :`Radius` (`self.RadiusOfAttack`) :`TraceChannel` "TraceTypeQuery3" :`DrawDebugType` "ForOneFrame"))
  (if _returnvalue_3
    (bind (_bblockinghit _binitialoverlap _time _distance _location _impactpoint _normal _impactnormal _physmat _hitactor) (`GameplayStatics.BreakHitResult` _outhit))
    (if (and (== _hitactor _returnvalue) (not (`KismetArrayLibrary.Array_Contains` (`self.DamagedActors`) _returnvalue)))
      (message `/Game/Blueprints/Interfaces/BPI_Damageable.TakeDamage` _hitactor (`self.Damage`) self)
      (`KismetArrayLibrary.Array_AddUnique` (`self.DamagedActors`) _hitactor))))

(event `Attack`
  ; Attack Logic
  ;; Attack Logic
  (`KismetArrayLibrary.Array_Clear` (`self.DamagedActors`))
  (`|PlayMontage` (`self.Mesh`) (`self.AttackMontage`)
    (:`OnCompleted`
      _)
    (:`OnInterrupted`
      _))
  (`self.OnAttackEnd`))

(event `UpdateHUDHealthBar`
  (params (CurrentHealthPercentage :type "Float (double-precision)") (CurrentHealth :type "Float (double-precision)") (MaximumHealth :type "Float (double-precision)"))
  ; Update HealthBar
  (bind _hudwidget (`self.HUDWidget`)
    (:`then`
      (`/Game/UI/WB_Enemy.UpdateHealthBar` _hudwidget CurrentHealthPercentage))
    (:`else`)))

(event `self.ReceiveTick`
  (params (DeltaSeconds :type "Float (single-precision)"))
  ; Tick
  (`self.RotateHealthBarTowardsCamera`))

(fn `BindUIEvents`
  (bind _bpc_healthcomponent (`self.BPC_HealthComponent`)
    (:`then`
      (add `/Game/Blueprints/Components/BPC_HealthComponent.On Health Update` _bpc_healthcomponent (`|CreateDelegate` :!event `UpdateHUDHealthBar`))
      (add `/Game/Blueprints/Components/BPC_HealthComponent.On Ready` _bpc_healthcomponent (`|CreateDelegate` :!event `InitializeHealthBar`))
      (`/Game/Blueprints/Components/BPC_HealthComponent.Init` _bpc_healthcomponent)
      (add `/Game/Blueprints/Components/BPC_HealthComponent.On Death` _bpc_healthcomponent (`|CreateDelegate` :!event `Death`)))
    (:`else`)))

(fn `GetPatrolRoute`
  (returns (PatrolRoute :type "/Game/Blueprints/Enemies/AI/BP_Patrol_Route Object Reference"))
  (return (`self.PatrolRoute`)))

(fn `InitializeHealthBar`
  (params (HealthComoponent :type "/Game/Blueprints/Components/BPC_HealthComponent Object Reference"))
  (bind _health_percentage (`/Game/Blueprints/Components/BPC_HealthComponent.Get Current Health Percent` HealthComoponent))
  (`self.UpdateHUDHealthBar` _health_percentage))

(fn `RotateHealthBarTowardsCamera`
  (`/Engine/EditorBlueprintResources/StandardMacros.IsValid` (`self.Widget`)
    (:`Is Valid`
      (`SceneComponent.K2_SetWorldRotation` (`self.Widget`) (`KismetMathLibrary.FindLookAtRotation` (`SceneComponent.K2_GetComponentLocation` (`self.Widget`)) (`SceneComponent.K2_GetComponentLocation` (`PlayerCameraManager.TransformComponent` (`GameplayStatics.GetPlayerCameraManager` 0)))) false false))))

(fn `SetMovementSpeed`
  (params (Speed :type "/Game/Blueprints/Enums/E_MovementSpeed Enum" :default "NewEnumerator0"))
  (returns (SpeedValue :type "Float (double-precision)"))
  (bind _output_get (set `CharacterMovementComponent.MaxWalkSpeed` (select `/Game/Blueprints/Enums/E_MovementSpeed` Speed :`NewEnumerator0` (`self.Idle`) :`NewEnumerator1` (`self.Walk`) :`NewEnumerator2` (`self.Run`)) (`self.CharacterMovement`)))
  (return _output_get))

(fn `UserConstructionScript`)