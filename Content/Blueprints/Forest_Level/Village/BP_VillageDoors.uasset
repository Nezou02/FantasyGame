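; BP_VillageDoors is a village double door that swings open when the player character enters its Box trigger.
; The overlap plays two timelines together, each interpolating the yaw of one door mesh in opposite directions.
; During left-door updates, a DoOnce disables the invisible wall's collision once both tracks read at or below 0.5.
; The graph contains no closing logic.
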(event `self.Box.OnComponentBeginOverlap`
  (params (OverlappedComponent :type "PrimitiveComponent Object Reference") (OtherActor :type "Actor Object Reference") (OtherComp :type "PrimitiveComponent Object Reference") (OtherBodyIndex :type Integer) (bFromSweep :type Boolean) (SweepResult :type "HitResult Structure (by ref)"))
  (if (== OtherActor (`GameplayStatics.GetPlayerCharacter` 0))
    (`|ExecutionSequence`
      (:`then_0`
        (bind (_direction _newtrack_0) (`Timeline|Timeline_Left_Door`)
          (:`Update`
            (`SceneComponent.K2_SetRelativeRotation` (`self.Left_Door_SM`) (`KismetMathLibrary.MakeRotator` 0.0 0.0 (`KismetMathLibrary.Lerp` 190.0 290.0 _newtrack_0)) false false)
            (if (and (<= _newtrack_0 0.5) (<= (stale _newtrack_0_2) 0.5))
              (`/Engine/EditorBlueprintResources/StandardMacros.DoOnce` false
                (:`Completed`
                  (`PrimitiveComponent.SetCollisionEnabled` (`self.Box_InvisibleWall`) "NoCollision")))))))
      (:`then_1`
        (bind (_direction_2 _newtrack_0_2) (`Timeline|Timeline_Rigth_Door`)
          (:`Update`
            (`SceneComponent.K2_SetRelativeRotation` (`self.Right_Door_SM`) (`KismetMathLibrary.MakeRotator` 0.0 0.0 (`KismetMathLibrary.Lerp` 12.0 -88.0 _newtrack_0_2)) false false)))))))

(fn `UserConstructionScript`)