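; Player controller that adds the player's Enhanced Input mapping context and creates the HUD widget on possess.
; It then caches the player character and binds to the update and ready events of its health and mana components.
; HUD update events push percent, current and maximum values to the bars and displays, with initialize functions supplying starting values from each component.
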(event `Update HUD Health Bar`
  (params (`Current Health Percent` :type "Float (double-precision)") (`Current Health` :type "Float (double-precision)") (`Maximum Health` :type "Float (double-precision)"))
  (bind _hud_widget (`self.HUD Widget`))
  ;[0.15 0.15 0.15 0.502] Event Which Calls HUD's Update Health Bar Function
  (`/Engine/EditorBlueprintResources/StandardMacros.IsValid` _hud_widget
    (:`Is Valid`
      (`/Game/UI/WB_HUD.Update Health Bar` _hud_widget `Current Health Percent`)
      (`/Game/UI/WB_HUD.Update Health Display` _hud_widget `Current Health` `Maximum Health`))))

(event `self.ReceivePossess`
  (params (PossessedPawn :type "Pawn Object Reference"))
  (`|ExecutionSequence`
    (:`then_0`
      ; Enabling Mapping Context
      (`EnhancedInputSubsystemInterface.AddMappingContext` (subsystem `EnhancedInputLocalPlayerSubsystem`) "/Game/Input/IMC/IMC_Player.IMC_Player" 0 (struct)))
    (:`then_1`
      ;[0.15 0.15 0.15 0.502] Enabling Player HUD (UI)
      (bind _returnvalue (`|CreateWidget` "/Game/UI/WB_HUD.WB_HUD_C" self))
      (bind _output_get (set `self.HUD Widget` _returnvalue))
      (`UserWidget.AddToViewport` _output_get 0)
      (`self.Sync Player Attributes With UI`))))

(event `Update HUD Mana Bar`
  (params (`Current Mana Percent` :type "Float (double-precision)") (`Current Mana` :type "Float (double-precision)") (`Maximum Mana` :type "Float (double-precision)"))
  (bind _hud_widget (`self.HUD Widget`))
  ;[0.15 0.15 0.15 0.502] Event Which Calls HUD's Update Mana Bar Function
  (`/Engine/EditorBlueprintResources/StandardMacros.IsValid` _hud_widget
    (:`Is Valid`
      (`/Game/UI/WB_HUD.Update Mana Bar` _hud_widget `Current Mana Percent`)
      (`/Game/UI/WB_HUD.Update Mana Display` _hud_widget `Current Mana` `Maximum Mana`))))

(fn `Bind UI Events`
  (params (`Player Health Component` :type "/Game/Blueprints/Components/BPC_HealthComponent Object Reference") (`Player Mana Component` :type "/Game/Blueprints/Components/BPC_ManaComponent Object Reference"))
  (`|ExecutionSequence`
    (:`then_0`
      (add `/Game/Blueprints/Components/BPC_HealthComponent.On Health Update` `Player Health Component` (`|CreateDelegate` :!event `Update HUD Health Bar`))
      (add `/Game/Blueprints/Components/BPC_HealthComponent.On Ready` `Player Health Component` (`|CreateDelegate` :!event `Initialize Health Bar`)))
    (:`then_1`
      (add `/Game/Blueprints/Components/BPC_ManaComponent.On Mana Update` `Player Mana Component` (`|CreateDelegate` :!event `Update HUD Mana Bar`))
      (add `/Game/Blueprints/Components/BPC_ManaComponent.On Ready` `Player Mana Component` (`|CreateDelegate` :!event `Initialize Mana Bar`)))))

(fn `Initialize Health Bar`
  (params (`Player Health Component` :type "/Game/Blueprints/Components/BPC_HealthComponent Object Reference"))
  (bind _health_percentage (`/Game/Blueprints/Components/BPC_HealthComponent.Get Current Health Percent` `Player Health Component`))
  (`self.Update HUD Health Bar` _health_percentage (`/Game/Blueprints/Components/BPC_HealthComponent.Current Health` `Player Health Component`) (`/Game/Blueprints/Components/BPC_HealthComponent.Maximum Health` `Player Health Component`)))

(fn `Initialize Mana Bar`
  (params (`Player Mana Component` :type "/Game/Blueprints/Components/BPC_ManaComponent Object Reference"))
  (bind _mana_percentage (`/Game/Blueprints/Components/BPC_ManaComponent.Get Current Mana Percentage` `Player Mana Component`))
  (`self.Update HUD Mana Bar` _mana_percentage (`/Game/Blueprints/Components/BPC_ManaComponent.Current Mana` `Player Mana Component`) (`/Game/Blueprints/Components/BPC_ManaComponent.Maxiumum Mana` `Player Mana Component`)))

(fn `Sync Player Attributes With UI`
  ; Bind Character Attribute Change Events To Keep UI Bars In Sync With Gameplay State And Initialize Attribute Bars
  (bind _asbp_player_character (cast `/Game/Blueprints/Player/BP_PlayerCharacter` (`GameplayStatics.GetPlayerPawn` 0)))
  (bind _output_get (set `self.Possessed Character` _asbp_player_character))
  (set `self.Player Health Coponent` (`/Game/Blueprints/Player/BP_PlayerCharacter.BPC_HealthCoponent` _output_get))
  (set `self.Player Mana Component` (`/Game/Blueprints/Player/BP_PlayerCharacter.BPC_ManaComponent` _output_get))
  (if (and (`KismetSystemLibrary.IsValid` (`self.Player Health Coponent`)) (`KismetSystemLibrary.IsValid` (`self.Player Mana Component`)))
    (`self.Bind UI Events` (`self.Player Health Coponent`) (`self.Player Mana Component`))))

(fn `UserConstructionScript`)