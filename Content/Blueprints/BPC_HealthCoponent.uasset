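; Actor component that tracks an owner's current and maximum health.
; DecreaseHealth and IncreaseHealth adjust the value, clamping it at zero and at MaxHealth respectively.
; After each change it broadcasts OnHealthUpdate with the health fraction from GetCurrentHealthPercent, so listeners can react without polling.
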(fn `Decrease Health`
  (params (Damage :type "Float (double-precision)"))
  (bind _output_get (set `self.Current Health` (- (`self.Current Health`) Damage)))
  (if (<= _output_get 0.0)
    (set `self.Current Health` 0.0))
  (bind _health_percentage (`self.Get Current Health Percent`))
  (`self.On Health Update` _health_percentage))

(fn `Get Current Health Percent`
  (returns (`Health Percentage` :type "Float (double-precision)"))
  (return (/ (`self.Current Health`) (`self.Max Health`))))

(fn `Increase Health`
  (params (Incrementation :type "Float (double-precision)"))
  (bind _output_get (set `self.Current Health` (+ (`self.Current Health`) Incrementation)))
  (if (> _output_get (`self.Max Health`))
    (set `self.Current Health` (`self.Max Health`)))
  (bind _health_percentage (`self.Get Current Health Percent`))
  (`self.On Health Update` _health_percentage))