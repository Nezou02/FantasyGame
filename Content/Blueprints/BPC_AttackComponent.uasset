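; BPC_AttackComponent is an actor component meant to handle basic attacks for its owner.
; On BeginPlay it caches the owner's BPC_HealthComponent and BPC_ManaComponent.
; BasicAttack checks that the owner is alive and CanAttack is set, then validates the mana component, with no attack logic beyond that check.
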(event `self.ReceiveBeginPlay`
  (bind _returnvalue (`self.GetOwner`))
  (set `self.Health Component` (`Actor.GetComponentByClass` _returnvalue "/Game/Blueprints/BPC_HealthComponent.BPC_HealthComponent_C"))
  (set `self.Mana Component` (`Actor.GetComponentByClass` _returnvalue "/Game/Blueprints/BPC_ManaComponent.BPC_ManaComponent_C")))

(event `Basic Attack`
  (bind _is_alive (`/Game/Blueprints/BPC_HealthComponent.Is Alive` (`self.Health Component`)))
  (if (and _is_alive (`self.Can Attack`))
    (`/Engine/EditorBlueprintResources/StandardMacros.IsValid` (`self.Mana Component`))))