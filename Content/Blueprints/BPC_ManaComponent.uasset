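; Mana component that tracks its owner's mana pool, starting full and broadcasting OnReady at BeginPlay.
; DecreaseMana subtracts mana with a floor of zero, then starts regeneration if below maximum and not already regenerating.
; A looping timer adds mana each interval, clamped to the maximum, and clears itself when full.
; Each decrease and regen tick broadcasts OnManaUpdate with percentage, current and maximum values for listeners.
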(event `self.ReceiveBeginPlay`
  (set `self.Current Mana` (`self.Maxiumum Mana`))
  (`self.On Ready` self))

(event `Start Mana Regeneration`
  ; Mana Regeneration Logic
  (set `self.Regeneration is Active` true)
  (bind _returnvalue (`KismetSystemLibrary.K2_SetTimerDelegate` (delegate `Regenerate Mana`) (`self.Regen Interval`) true)))

(event `Stop Regeneration`
  ; Mana Regeneration Logic
  (`KismetSystemLibrary.K2_ClearAndInvalidateTimerHandle` (stale `Start Mana Regeneration` _returnvalue))
  (set `self.Regeneration is Active` false))

(event `Regenerate Mana`
  ; Mana Regeneration Logic
  (bind _output_get (set `self.Current Mana` (`KismetMathLibrary.FClamp` (+ (`self.Current Mana`) (`self.Mana Regeneration`)) 0.0 (`self.Maxiumum Mana`))))
  (bind _mana_percentage (`self.Get Current Mana Percentage`))
  (`self.On Mana Update` _mana_percentage (`self.Current Mana`) (`self.Maxiumum Mana`))
  (if (== _output_get (`self.Maxiumum Mana`))
    (`self.Stop Regeneration`)))

(fn `Decrease Mana`
  (params (Decrementation :type "Float (double-precision)"))
  (bind _output_get (set `self.Current Mana` (- (`self.Current Mana`) Decrementation)))
  (if (< _output_get 0.0)
    (set `self.Current Mana` 0.0))
  (bind _mana_percentage (`self.Get Current Mana Percentage`))
  (`self.On Mana Update` _mana_percentage (`self.Current Mana`) (`self.Maxiumum Mana`))
  (`self.Handle Mana Regen`))

(fn `Get Current Mana Percentage`
  (returns (`Mana Percentage` :type "Float (double-precision)"))
  (return (/ (`self.Current Mana`) (`self.Maxiumum Mana`))))

(fn `Handle Mana Regen`
  (if (and (!= (`self.Current Mana`) (`self.Maxiumum Mana`)) (not (`self.Regeneration is Active`)))
    (`self.Start Mana Regeneration`)))