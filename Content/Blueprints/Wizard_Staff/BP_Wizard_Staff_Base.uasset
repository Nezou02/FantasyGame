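; Base wizard staff actor that fires projectiles when its ShootProjectile event is called with a rotation.
; It spawns the configured projectile class at the SpawnPoint location, owned by the staff, passing in its speed and damage.
; The staff mesh ignores the new projectile when moving, and an owning BP_PlayerCharacter is told to ignore it too.
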(event `Shoot Projectile`
  (params (Rotation :type "Rotator Structure"))
  (bind _returnvalue_location (`KismetMathLibrary.BreakTransform` (`SceneComponent.K2_GetComponentToWorld` (`self.Spawn Point`))))
  ; Shoot Projectile
  (bind _returnvalue (`|SpawnActorFromClass` (`self.Projectile Type`) (`KismetMathLibrary.MakeTransform` _returnvalue_location Rotation) "AlwaysSpawn" "MultiplyWithRoot" self 0.0 (`self.Projectile Speed`) (`self.Damage`) null))
  (`PrimitiveComponent.IgnoreActorWhenMoving` (`self.StaticMesh`) _returnvalue true)
  (bind _asbp_player_character (cast `/Game/Blueprints/Player/BP_PlayerCharacter` (`self.GetOwner`)))
  (`/Game/Blueprints/Player/BP_PlayerCharacter.Ignore Projectile` _asbp_player_character _returnvalue))

(fn `UserConstructionScript`)