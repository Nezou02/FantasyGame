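; BPC_AttackComponent is an actor component that gates its owner's basic attack on life state, readiness and mana.
; At BeginPlay it caches the owner's health and mana components.
; BasicAttack requires a living owner, CanAttack and a valid mana component with enough mana, then spends the cost, locks attacking and fires the OnBasicAttack dispatcher.
; ResetAttack re-enables attacking and is not called within this component.
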(event `self.ReceiveBeginPlay`
  (bind _returnvalue (`self.GetOwner`))
  (set `self.Health Component` (`Actor.GetComponentByClass` _returnvalue "/Game/Blueprints/Components/BPC_HealthComponent.BPC_HealthComponent_C"))
  (set `self.Mana Component` (`Actor.GetComponentByClass` _returnvalue "/Game/Blueprints/Components/BPC_ManaComponent.BPC_ManaComponent_C")))

(event `Basic Attack`
  (bind _mana_component (`self.Mana Component`))
  (bind _is_dead (`/Game/Blueprints/Components/BPC_HealthComponent.Is Entity Dead` (`self.Health Component`)))
  (if (and (not _is_dead) (`self.Can Attack`))
    (`/Engine/EditorBlueprintResources/StandardMacros.IsValid` _mana_component
      (:`Is Valid`
        (bind _enough (`/Game/Blueprints/Components/BPC_ManaComponent.Has Enough Mana` _mana_component (`self.Basic Attack Mana Cost`)))
        (if _enough
          (`/Game/Blueprints/Components/BPC_ManaComponent.Decrease Mana` _mana_component (`self.Basic Attack Mana Cost`))
          (set `self.Can Attack` false)
          (`self.On Basic Attack`))))))

(fn `Reset Attack`
  (set `self.Can Attack` true))