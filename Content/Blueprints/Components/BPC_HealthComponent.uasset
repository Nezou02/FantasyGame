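; Health component that tracks current and maximum health for its owning actor.
; On BeginPlay it fills health to maximum and broadcasts OnReady with itself.
; Decrease and Increase functions clamp health, broadcast OnHealthUpdate with the new percentage, and ignore changes once dead.
; Reaching zero latches the dead flag and fires OnDeath before the final update; helpers expose percentage and dead state.
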(event `self.ReceiveBeginPlay`
  (set `self.Current Health` (`self.Maximum Health`))
  (`self.On Ready` self))

(fn `Decrease Health`
  (params (Damage :type "Float (double-precision)"))
  (if (not (`self.Is Dead`))
    (bind _output_get (set `self.Current Health` (- (`self.Current Health`) Damage)))
    (if (<= _output_get 0.0)
      (set `self.Current Health` 0.0)
      (set `self.Is Dead` true)
      (`self.On Death`))
    (bind _health_percentage (`self.Get Current Health Percent`))
    (`self.On Health Update` _health_percentage (`self.Current Health`) (`self.Maximum Health`))))

(fn `Get Current Health Percent`
  (returns (`Health Percentage` :type "Float (double-precision)"))
  (return (/ (`self.Current Health`) (`self.Maximum Health`))))

(fn `Increase Health`
  (params (Incrementation :type "Float (double-precision)"))
  (if (not (`self.Is Dead`))
    (bind _output_get (set `self.Current Health` (+ (`self.Current Health`) Incrementation)))
    (if (> _output_get (`self.Maximum Health`))
      (set `self.Current Health` (`self.Maximum Health`)))
    (bind _health_percentage (`self.Get Current Health Percent`))
    (`self.On Health Update` _health_percentage (`self.Current Health`) (`self.Maximum Health`))))

(fn `Is Entity Dead`
  (returns (`Is Dead` :type Boolean))
  (return (`self.Is Dead`)))